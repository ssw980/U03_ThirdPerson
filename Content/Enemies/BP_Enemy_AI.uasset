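; Enemy character Blueprint that shows its controller's name and carries a great sword.
; On BeginPlay it runs the parent logic, then sets the ControllerName text to the object name of its controller.
; It then attaches the GreatSword component to the "ee" socket on the Mesh, keeping relative transforms.
; The construction script only calls the parent, and the file itself contains no AI decision logic.
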(event `self.ReceiveBeginPlay`
  (`parent.ReceiveBeginPlay`)
  (`TextRenderComponent.K2_SetText` (`self.ControllerName`) (`KismetTextLibrary.Conv_StringToText` (`KismetSystemLibrary.GetObjectName` (`self.GetController`))))
  (`self.K2_AttachToComponent` (`self.GreatSword`) (`self.Mesh`) "ee" "KeepRelative" "KeepRelative" "KeepRelative" true))

(fn `UserConstructionScript`
  (`parent.UserConstructionScript`))