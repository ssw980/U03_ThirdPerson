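; Warp skill for a magic character that teleports its owner to the point under the mouse cursor on static world geometry.
; While equipped, Tick moves a decal and mesh marker to the cursor hit, aligning the decal to the surface normal.
; Spell stores the target, locks movement and plays a montage, or ends the attack without a hit.
; A separate Warp event performs the teleport at fixed height; EndSpell restores movement.
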(event `self.ReceiveBeginPlay`
  (`parent.ReceiveBeginPlay`)
  (`SceneComponent.SetVisibility` (`self.Decal`) false false)
  (`SceneComponent.SetVisibility` (`self.StaticMesh`) false false))

(event `self.OnEquippedSkill`
  (`parent.OnEquippedSkill`)
  (set `self.Equipped` true))

(event `self.OnUnEquippedSkill`
  (`parent.OnUnEquippedSkill`)
  (set `self.Equipped` false))

(event `Warp`
  (if (`self.CanWarp`)
    (set `self.CanWarp` false)
    (`self.K2_SetActorLocation` (`self.GetOwnerToCharacter`) (`KismetMathLibrary.MakeVector` (.x (`self.WarpLocation`)) (.y (`self.WarpLocation`)) 150.0) false true)))

(event `self.Spell`
  (`parent.Spell`)
  (bind _location (`self.GetCursorLocation`)
    (:`True`
      (set `self.WarpLocation` _location)
      (set `self.CanWarp` true)
      (`/Game/Weapons/BP_Weapon.SetCanMove` (`self.Get Owner to Magic`) false)
      (`Character.PlayAnimMontage` (`self.GetOwnerToCharacter`) "/Game/Character/Montages/MG_Warp_Montage.MG_Warp_Montage" 2.0 "None"))
    (:`False`
      (`/Game/Weapons/BP_Weapon.EndAttack` (`self.Get Owner to Magic`))
      (set `self.CanWarp` false))))

(event `self.ReceiveTick`
  (params (DeltaSeconds :type "Float (single-precision)"))
  (if (`self.Equipped`)
    (bind (_location _impactpoint) (`self.GetCursorLocation`)
      (:`True`
        (`SceneComponent.K2_SetWorldLocation` (`self.Decal`) _location false false)
        (`SceneComponent.K2_SetWorldLocation` (`self.StaticMesh`) _location false false)
        (`SceneComponent.K2_SetWorldRotation` (`self.Decal`) (`KismetMathLibrary.Conv_VectorToRotator` _impactpoint) false false)
        (`SceneComponent.SetVisibility` (`self.Decal`) true false)
        (`SceneComponent.SetVisibility` (`self.StaticMesh`) true false))
      (:`False`
        (`SceneComponent.SetVisibility` (`self.Decal`) false false :!label _label)
        (`SceneComponent.SetVisibility` (`self.StaticMesh`) false false)))
    (else
      (goto _label))))

(event `self.EndSpell`
  (`parent.EndSpell`)
  (`/Game/Weapons/BP_Weapon.SetCanMove` (`self.Get Owner to Magic`) true))

(fn `UserConstructionScript`
  (`parent.UserConstructionScript`))