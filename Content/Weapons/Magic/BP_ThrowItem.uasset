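; BP_ThrowItem is a base thrown magic projectile that self-destructs after a short lifespan.
; It resolves its owner chain through BP_Skill_Throw up to the owning BP_Magic.
; SendDamage spawns an impact particle oriented from the caster toward the hit actor, forwards the damage to BP_Magic, then destroys the projectile.
; No collision or movement logic appears here, only this damage helper.
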(event `self.ReceiveBeginPlay`
  (`self.SetLifeSpan` 4.0))

(fn `GetOwnerToMagic`
  (returns (`AsBP Magic` :type "/Game/Weapons/Magic/BP_Magic Object Reference"))
  (bind _asbp_magic (cast `/Game/Weapons/Magic/BP_Magic` (`self.GetOwner` (`self.GetOwnerToThrow`))))
  (return _asbp_magic))

(fn `GetOwnerToThrow`
  (returns (`AsBP Skill Throw` :type "/Game/Weapons/Magic/BP_Skill_Throw Object Reference"))
  (bind _asbp_skill_throw (cast `/Game/Weapons/Magic/BP_Skill_Throw` (`self.GetOwner`)))
  (return _asbp_skill_throw))

(fn `SendDamage`
  (params (OtherActor :type "Actor Object Reference") (Damage :type "Float (double-precision)" :default 20.0) (ImpactParticle :type "ParticleSystem Object Reference") (ImpactParticleOffset :type "Vector Structure") (ImpactParticleScale :type "Vector Structure" :default (1.0 1.0 1.0)))
  (`GameplayStatics.SpawnEmitterAtLocation` (`local.ImpactParticle`) (+ (`self.K2_GetActorLocation`) (`local.ImpactParticleOffset`)) (`KismetMathLibrary.FindLookAtRotation` (`self.K2_GetActorLocation` (`self.GetOwner` (`self.GetOwnerToMagic`))) (`self.K2_GetActorLocation` (`local.OtherActor`))) (`local.ImpactParticleScale`))
  (`/Game/Weapons/BP_Weapon.SendDamage` (`self.GetOwnerToMagic`) (`local.OtherActor`) (`local.Damage`))
  (`self.K2_DestroyActor`))

(fn `UserConstructionScript`)