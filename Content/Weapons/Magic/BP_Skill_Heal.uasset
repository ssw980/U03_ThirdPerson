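; BP_Skill_Heal is a magic skill that heals its owning character when cast.
; On Spell it calls the parent, keeps or restores the caster's movement through the magic owner, and plays a buff montage on the character.
; It then raises health by a fixed amount through the owner's StatusComponent, if one exists.
; EndSpell calls the parent and enables movement again.
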(event `self.Spell`
  (bind _returnvalue (`self.GetComponentByClass` (`self.GetOwnerToCharacter`) "/Game/Components/StatusComponent.StatusComponent_C"))
  (`parent.Spell`)
  (`/Game/Weapons/BP_Weapon.SetCanMove` (`self.Get Owner to Magic`) true)
  (`Character.PlayAnimMontage` (`self.GetOwnerToCharacter`) "/Game/Character/Montages/MG_Buff_Montage.MG_Buff_Montage" 1.0 "None")
  (`/Engine/EditorBlueprintResources/StandardMacros.IsValid` _returnvalue
    (:`Is Valid`
      (`/Game/Components/StatusComponent.Increase Health` _returnvalue 20.0))))

(event `self.EndSpell`
  (`parent.EndSpell`)
  (`/Game/Weapons/BP_Weapon.SetCanMove` (`self.Get Owner to Magic`) true))

(fn `UserConstructionScript`
  (`parent.UserConstructionScript`))