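; BP_Skill is a skeleton for a magic skill owned by a BP_Magic, with equip, unequip, spell and end-spell events.
; Equipping re-enables movement on the magic and sets its idling state message; the other events are empty.
; Helper functions resolve the ownership chain, casting the owner to BP_Magic and that magic's owner to Character.
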(event `OnEquippedSkill`
  (bind _asbp_magic (`self.Get Owner to Magic`))
  (`/Game/Weapons/BP_Weapon.SetCanMove` _asbp_magic true)
  (message `/Game/Interfaces/IState.SetStateIdling` _asbp_magic))

(event `Spell`)

(event `EndSpell`)

(event `OnUnEquippedSkill`)

(fn `Get Owner to Magic`
  (returns (`AsBP Magic` :type "/Game/Weapons/Magic/BP_Magic Object Reference"))
  (bind _asbp_magic (cast `/Game/Weapons/Magic/BP_Magic` (`self.GetOwner`)))
  (return _asbp_magic))

(fn `GetOwnerToCharacter`
  (returns (AsCharacter :type "Character Object Reference"))
  (bind _ascharacter (cast `Character` (`self.GetOwner` (`self.Get Owner to Magic`))))
  (return _ascharacter))

(fn `UserConstructionScript`)